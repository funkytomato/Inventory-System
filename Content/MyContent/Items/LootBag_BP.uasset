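; LootBag_BP is a loot bag actor that holds items in an InventorySystem component and removes itself once emptied.
; When the inventory updates and its quantity is zero or less, it removes the HUD's Menu widget through player 0's MyPlayerController, then destroys the actor.
; The cleanup only runs if the controller cast succeeds, and it is the only active logic, with no Tick or overlap handling.
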(event `self.InventorySystem.OnInventoryUpdated`
  (if (<= (`/Game/MyContent/Blueprints/InventorySystem/InventorySystem.GetQuantity` (`self.InventorySystem`)) 0)
    (bind _asmy_player_controller (cast `/Game/MyContent/Blueprints/Characters/MyPlayerController` (`GameplayStatics.GetPlayerController` 0)))
    (`Widget.RemoveFromParent` (`/Game/MyContent/UI/PlayerHUD_WBP.Menu` (`/Game/MyContent/Blueprints/Characters/MyPlayerController.HUD` _asmy_player_controller)))
    (`self.K2_DestroyActor`)))

(fn `UserConstructionScript`
  (`parent.UserConstructionScript`))