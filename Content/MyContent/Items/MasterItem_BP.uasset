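; Base item actor for world pickups that supplies a look-at prompt and records its removal in level save data.
; LookAt uses the ItemDataComponent's ItemID to find its data table row and returns "Pick up" plus the item's name.
; When destroyed, it adds itself uniquely to the ActorsRemoved list in the first-person game mode's level save data.
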(event `self.ReceiveDestroyed`
  (bind _asbp_first_person_game_mode (cast `/Game/MyContent/Blueprints/BP_FirstPersonGameMode` (`GameplayStatics.GetGameMode`)))
  (`KismetArrayLibrary.Array_AddUnique` (`/Game/MyContent/Blueprints/SaveData_Level.ActorsRemoved` (`/Game/MyContent/Blueprints/BP_FirstPersonGameMode.As Save Data Level` _asbp_first_person_game_mode)) (`|ConvertAsset` self)))

(fn `LookAt`
  (returns (message :type Text))
  (bind (_itemid_datatable _itemid_rowname) (break `DataTableRowHandle` (`/Game/MyContent/Blueprints/InventorySystem/ItemDataComponent.ItemID` (`self.ItemDataComponent`))))
  (bind _returnvalue (`|GetDataTableRow` _itemid_datatable _itemid_rowname)
    (:`then`
      (return (`|FormatText` "Pick up {item}" (`.Name_2_1BB1B690D24936795004B5B291128681` (break `/Game/MyContent/Blueprints/InventorySystem/Data/FItemStruct` _returnvalue)))))))

(fn `UserConstructionScript`)